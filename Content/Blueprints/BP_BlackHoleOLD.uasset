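; Black hole actor that pulls in nearby physics objects and destroys what reaches its core.
; Each Tick, it queries the outer sphere for PhysicsBody components and applies an inward radial force to those simulating physics.
; The pull uses negative strength with constant falloff as an acceleration change, so it ignores mass and distance within the radius.
; Any actor that begins overlapping the inner sphere is destroyed, with no filtering.
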(event `self.ReceiveTick`
  (params (DeltaSeconds :type "Float (single-precision)"))
  (bind _returnvalue (`self.GetTransform`))
  (bind _outerspherecollider (`self.OuterSphereCollider`))
  (bind _outcomponents (`KismetSystemLibrary.ComponentOverlapComponents` _outerspherecollider _returnvalue (`|MakeArray` "ObjectTypeQuery4" :!type "EObjectTypeQuery Enum")))
  (for _array_element _outcomponents
    (if (`SceneComponent.IsSimulatingPhysics` _array_element "None")
      (`PrimitiveComponent.AddRadialForce` _array_element (`KismetMathLibrary.TransformLocation` _returnvalue) (`SphereComponent.GetScaledSphereRadius` _outerspherecollider) -2000.0 "RIF_Constant" true))))

(event `self.InnerSphereCollider.OnComponentBeginOverlap`
  (params (OverlappedComponent :type "PrimitiveComponent Object Reference") (OtherActor :type "Actor Object Reference") (OtherComp :type "PrimitiveComponent Object Reference") (OtherBodyIndex :type Integer) (bFromSweep :type Boolean) (SweepResult :type "HitResult Structure (by ref)"))
  (`self.K2_DestroyActor` OtherActor))

(fn `UserConstructionScript`)