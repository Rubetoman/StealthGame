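; BP_LaunchPadOld is a launch pad that throws characters and physics objects when they overlap its box collider.
; The launch direction is the overlapping actor's own facing with a pitch angle added, scaled by a strength variable.
; Characters are launched with LaunchCharacter, overriding their current velocity.
; Other components receive a velocity-change impulse only if they simulate physics.
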(event `self.BoxCollider.OnComponentBeginOverlap`
  (params (OverlappedComponent :type "PrimitiveComponent Object Reference") (OtherActor :type "Actor Object Reference") (OtherComp :type "PrimitiveComponent Object Reference") (OtherBodyIndex :type Integer) (bFromSweep :type Boolean) (SweepResult :type "HitResult Structure (by ref)"))
  (bind _returnvalue (* (`KismetMathLibrary.Conv_RotatorToVector` (`KismetMathLibrary.MakeRotator` (.roll (`self.K2_GetActorRotation` OtherActor)) (+ (`self.LaunchPitchAngle`) (.pitch (`self.K2_GetActorRotation` OtherActor))) (.yaw (`self.K2_GetActorRotation` OtherActor)))) (`self.LauchStrength`)))
  (bind _ascharacter (cast `Character` OtherActor)
    (:`then`
      (`Character.LaunchCharacter` _ascharacter _returnvalue true true))
    (:`CastFailed`
      (if (`SceneComponent.IsSimulatingPhysics` OtherComp "None")
        (`PrimitiveComponent.AddImpulse` OtherComp _returnvalue "None" true)))))

(fn `UserConstructionScript`)